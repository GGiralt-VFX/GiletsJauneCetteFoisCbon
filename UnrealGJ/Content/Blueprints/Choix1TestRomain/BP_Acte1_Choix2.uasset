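; BP_Acte1_Choix2 is a clickable choice actor in Act 1 of a branching choice sequence, apparently a test cylinder.
; On click, it passes two new choices, both BP_Acte1_Choix3, to the Acte 1 blueprint reference.
; It also updates the HUD's bottom text with a French line about clicking a cylinder, then destroys the current choices.
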(event `self.ReceiveBeginPlay`
  (`parent.ReceiveBeginPlay`))

(event `self.TouchClick.OnClicked`
  (params (TouchedComponent :type "PrimitiveComponent Object Reference") (ButtonPressed :type "Key Structure"))
  (`KismetSystemLibrary.PrintString` "Clique Cylindre")
  (bind _arrayactorref (`self.SetNewChoices` 2 "/Game/Blueprints/Choix1TestRomain/BP_Acte1_Choix3.BP_Acte1_Choix3_C" "/Game/Blueprints/Choix1TestRomain/BP_Acte1_Choix3.BP_Acte1_Choix3_C"))
  (message `/Game/Blueprints/BPI_test.GetReferences` (`self.BP_Acte1Ref`) _arrayactorref)
  (bind _text (`self.SetText` "Je viens de cliquer un cylindre"))
  (`/Game/Blueprints/HUDClassCustom.UpdateBottomText` (`self.HudReference`) _text)
  (`self.DestroyCurrentChoices`))

(fn `UserConstructionScript`
  (`parent.UserConstructionScript`))