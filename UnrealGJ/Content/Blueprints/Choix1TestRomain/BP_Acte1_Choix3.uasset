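; BP_Acte1_Choix3 is a clickable choice in Act 1, apparently a test version given its folder and placeholder text.
; On click it prints a debug string and sends the Act 1 reference a new set of three choices, all pointing to BP_Acte1_Choix1.
; It then updates the HUD's bottom text through HudReference and destroys the current choices.
; BeginPlay is disabled and the construction script only calls its parent.
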(event `self.TouchClick.OnClicked`
  (params (TouchedComponent :type "PrimitiveComponent Object Reference") (ButtonPressed :type "Key Structure"))
  (`KismetSystemLibrary.PrintString` "Clique Pipe")
  (bind _arrayactorref (`self.SetNewChoices` 3 "/Game/Blueprints/Choix1TestRomain/BP_Acte1_Choix1.BP_Acte1_Choix1_C" "/Game/Blueprints/Choix1TestRomain/BP_Acte1_Choix1.BP_Acte1_Choix1_C" "/Game/Blueprints/Choix1TestRomain/BP_Acte1_Choix1.BP_Acte1_Choix1_C"))
  (message `/Game/Blueprints/BPI_test.GetReferences` (`self.BP_Acte1Ref`) _arrayactorref)
  (bind _text (`self.SetText` "Je viens de cliquer une pipe"))
  (`/Game/Blueprints/HUDClassCustom.UpdateBottomText` (`self.HudReference`) _text)
  (`self.DestroyCurrentChoices`))

(fn `UserConstructionScript`
  (`parent.UserConstructionScript`))