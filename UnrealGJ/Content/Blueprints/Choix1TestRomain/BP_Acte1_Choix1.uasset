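; BP_Acte1_Choix1 is a clickable choice actor for Act 1, apparently a test in a branching-choice system.
; Clicking its TouchClick component passes a struct of two next choices, both BP_Acte1_Choix2, to the Act 1 blueprint reference.
; It then sends a French line about clicking a cube to the HUD's bottom text and destroys the current choices.
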(event `self.ReceiveBeginPlay`
  (`parent.ReceiveBeginPlay`))

(event `self.TouchClick.OnClicked`
  (params (TouchedComponent :type "PrimitiveComponent Object Reference") (ButtonPressed :type "Key Structure"))
  (`KismetSystemLibrary.PrintString` "Clique Cube")
  (bind _arrayactorref (`self.SetNewChoices` 2 "/Game/Blueprints/Choix1TestRomain/BP_Acte1_Choix2.BP_Acte1_Choix2_C" "/Game/Blueprints/Choix1TestRomain/BP_Acte1_Choix2.BP_Acte1_Choix2_C"))
  (message `/Game/Blueprints/BPI_test.GetReferences` (`self.BP_Acte1Ref`) _arrayactorref)
  (bind _text (`self.SetText` "Je viens de cliquer un cube"))
  (`/Game/Blueprints/HUDClassCustom.UpdateBottomText` (`self.HudReference`) _text)
  (`self.DestroyCurrentChoices`))

(fn `UserConstructionScript`
  (`parent.UserConstructionScript`))