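; Story choice Blueprint for Act 1, the "Ne pas réagir" (do not react) option at step 5 of a French branching narrative.
; Clicking it sets two follow-up choices, waiting or sending water, and passes them to the Act 1 reference.
; It then updates the HUD bottom text with the growing crowd and an insistent grandmother, and destroys the current choices.
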(event `self.ReceiveBeginPlay`
  (`parent.ReceiveBeginPlay`))

(event `self.TouchClick.OnClicked`
  (params (TouchedComponent :type "PrimitiveComponent Object Reference") (ButtonPressed :type "Key Structure"))
  (`KismetSystemLibrary.PrintString` "Clique Cube")
  (bind _arrayactorref (`self.SetNewChoices` 2 "/Game/Blueprints/6/BP_6_Attend.BP_6_Attend_C" "/Game/Blueprints/6/BP_6_EnvoyerEau.BP_6_EnvoyerEau_C"))
  (message `/Game/Blueprints/BPI_test.GetReferences` (`self.BP_Acte1Ref`) _arrayactorref)
  (bind _text (`self.SetText` "La foule devient de plus en plus nombreuse. Une mamie veut circuler et vient vous voir toutes les 30 secondes pour passer car ''Medor attend ses croquettes chez elle''"))
  (`/Game/Blueprints/HUDClassCustom.UpdateBottomText` (`self.HudReference`) _text)
  (`self.DestroyCurrentChoices`))

(fn `UserConstructionScript`
  (`parent.UserConstructionScript`))