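; BP_5_PlusFlash is a clickable choice actor in a branching French-language narrative, one step in the Act 1 story.
; On click it passes two follow-up choices, letting through or blocking a student medic street rescue team, to the Act 1 Blueprint.
; It then updates the HUD's bottom text with the wounded-and-rescuers situation and destroys the current choices.
; BeginPlay and construction only defer to the parent class.
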(event `self.ReceiveBeginPlay`
  (`parent.ReceiveBeginPlay`))

(event `self.TouchClick.OnClicked`
  (params (TouchedComponent :type "PrimitiveComponent Object Reference") (ButtonPressed :type "Key Structure"))
  (`KismetSystemLibrary.PrintString` "Clique Cube")
  (bind _arrayactorref (`self.SetNewChoices` 2 "/Game/Blueprints/6/BP_6_LaisserPasser.BP_6_LaisserPasser_C" "/Game/Blueprints/6/BP_6_EmpecherPasser.BP_6_EmpecherPasser_C"))
  (message `/Game/Blueprints/BPI_test.GetReferences` (`self.BP_Acte1Ref`) _arrayactorref)
  (bind _text (`self.SetText` "Certains sont gravement blessés. Une troupe de secours (de rue) composé d'étudiant en médecine, veulent passer pour leur porter secours  "))
  (`/Game/Blueprints/HUDClassCustom.UpdateBottomText` (`self.HudReference`) _text)
  (`self.DestroyCurrentChoices`))

(fn `UserConstructionScript`
  (`parent.UserConstructionScript`))