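; Clickable story-choice Blueprint for step 5 of an interactive narrative about an arrest during a protest.
; On click it fills the next two choices with the step 6 options, on the ground during the arrest or pushing back, through the Act 1 Blueprint reference.
; It then updates the HUD bottom text to say protesters intervene during the arrest and destroys the current choices.
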(event `self.ReceiveBeginPlay`
  (`parent.ReceiveBeginPlay`))

(event `self.TouchClick.OnClicked`
  (params (TouchedComponent :type "PrimitiveComponent Object Reference") (ButtonPressed :type "Key Structure"))
  (`KismetSystemLibrary.PrintString` "Clique Cube")
  (bind _arrayactorref (`self.SetNewChoices` 2 "/Game/Blueprints/6/BP_6_ATerreInterpeller.BP_6_ATerreInterpeller_C" "/Game/Blueprints/6/BP_6_Repousser.BP_6_Repousser_C"))
  (message `/Game/Blueprints/BPI_test.GetReferences` (`self.BP_Acte1Ref`) _arrayactorref)
  (bind _text (`self.SetText` "Des manifestants s'interposent durant l'interpellation "))
  (`/Game/Blueprints/HUDClassCustom.UpdateBottomText` (`self.HudReference`) _text)
  (`self.DestroyCurrentChoices`))

(fn `UserConstructionScript`
  (`parent.UserConstructionScript`))