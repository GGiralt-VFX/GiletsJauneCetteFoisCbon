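; BP_Choix is a choice actor with a TouchClick component, apparently a base for the choices offered in BP_Acte1.
; After a short delay for the HUD to spawn, BeginPlay caches the custom HUD and the BP_Acte1 actor.
; SetNewChoices refills that act's ArrayActorRef with up to four choices, and DestroyCurrentChoices destroys every BP_Choix.
; MoveRight slides TouchClick with easing, while click, touch and MoveLeft events are empty and SetText only echoes its input.
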(event `self.ReceiveBeginPlay`
  (`KismetSystemLibrary.Delay` 0.2) ; delay le temps que le HUD spawn
  (set `self.HUDReference` (cast `/Game/Blueprints/HUDClassCustom` (`PlayerController.GetHUD` (`GameplayStatics.GetPlayerController` 0)) :!pure true))
  (bind _outactors (`GameplayStatics.GetAllActorsOfClass` "/Game/Blueprints/BP_Acte1.BP_Acte1_C"))
  (for _array_element _outactors
    (set `self.BP_Acte1Ref` _array_element)))

(event `self.TouchClick.OnBeginCursorOver`
  (params (TouchedComponent :type "PrimitiveComponent Object Reference")))

(event `Move Right`
  (`KismetSystemLibrary.MoveComponentTo` (`self.TouchClick`) (0.0 800.0 0.0) (struct) true true 1.0)
  (`KismetSystemLibrary.Delay` 1.0))

(event `self.TouchClick.OnClicked`
  (params (TouchedComponent :type "PrimitiveComponent Object Reference") (ButtonPressed :type "Key Structure")))

(event `self.TouchClick.OnInputTouchBegin`
  (params (FingerIndex :type "ETouchIndex Enum" :default "Touch1") (TouchedComponent :type "PrimitiveComponent Object Reference")))

(event `Move Left`)

(fn `DestroyCurrentChoices`
  (bind _outactors (`GameplayStatics.GetAllActorsOfClass` "BP_Choix_C"))
  (for _array_element _outactors
    (`self.K2_DestroyActor` _array_element))
  (return))

(fn `SetNewChoices`
  (params (NumberOfChoicesFilled :type Integer) (Choix1 :type "Actor Class Reference") (Choix2 :type "Actor Class Reference") (Choix3 :type "Actor Class Reference") (Choix4 :type "Actor Class Reference"))
  (returns (ArrayActorRef :type "Array of Actor Class Reference"))
  (bind _arrayactorref (`/Game/Blueprints/BP_Acte1.ArrayActorRef` (`self.BP_Acte1Ref`)))
  (`|ExecutionSequence`
    (:`then_0`
      (`KismetArrayLibrary.Array_Clear` _arrayactorref))
    (:`then_1`
      (if (>= NumberOfChoicesFilled 1)
        (`KismetArrayLibrary.Array_Add` _arrayactorref Choix1)))
    (:`then_2`
      (if (>= NumberOfChoicesFilled 2)
        (`KismetArrayLibrary.Array_Add` _arrayactorref Choix2)))
    (:`then_3`
      (if (>= NumberOfChoicesFilled 3)
        (`KismetArrayLibrary.Array_Add` _arrayactorref Choix3)))
    (:`then_4`
      (if (>= NumberOfChoicesFilled 4)
        (`KismetArrayLibrary.Array_Add` _arrayactorref Choix4)))
    (:`then_5`
      (return _arrayactorref))))

(fn `SetText`
  (params (BottomText :type Text))
  (returns (Text :type Text))
  (return BottomText))

(fn `UserConstructionScript`)