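; BP_4_LacFlash is a clickable choice node in a branching narrative, apparently part of Act 1.
; On touch click it builds a set of two follow-up choices, BP_5_Interpeller3 and BP_5_MattGroupeGO, and passes it to the Act 1 Blueprint.
; It then updates the HUD's bottom text with a French story line and destroys the current choices.
; BeginPlay and construction defer to the parent class.
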(event `self.ReceiveBeginPlay`
  (`parent.ReceiveBeginPlay`))

(event `self.TouchClick.OnClicked`
  (params (TouchedComponent :type "PrimitiveComponent Object Reference") (ButtonPressed :type "Key Structure"))
  (`KismetSystemLibrary.PrintString` "Clique Cube")
  (bind _arrayactorref (`self.SetNewChoices` 2 "/Game/Blueprints/5/BP_5_Interpeller3.BP_5_Interpeller3_C" "/Game/Blueprints/5/BP_5_MattGroupeGO.BP_5_MattGroupeGO_C"))
  (message `/Game/Blueprints/BPI_test.GetReferences` (`self.BP_Acte1Ref`) _arrayactorref)
  (bind _text (`self.SetText` "3 personnes brulent une poubelle en signe de rispote"))
  (`/Game/Blueprints/HUDClassCustom.UpdateBottomText` (`self.HudReference`) _text)
  (`self.DestroyCurrentChoices`))

(fn `UserConstructionScript`
  (`parent.UserConstructionScript`))