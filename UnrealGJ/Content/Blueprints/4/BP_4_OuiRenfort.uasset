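; Choice actor for a branching narrative scene, the "yes, reinforcements" option at step 4.
; Clicking it registers two follow-up choices, encircle or send Matt's group, through the Act 1 blueprint reference.
; It then updates the HUD bottom text to announce arriving reinforcements and protesters splitting into two groups, and destroys the current choices.
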(event `self.ReceiveBeginPlay`
  (`parent.ReceiveBeginPlay`))

(event `self.TouchClick.OnClicked`
  (params (TouchedComponent :type "PrimitiveComponent Object Reference") (ButtonPressed :type "Key Structure"))
  (`KismetSystemLibrary.PrintString` "Clique Cube")
  (bind _arrayactorref (`self.SetNewChoices` 2 "/Game/Blueprints/5/BP_5_Encercler.BP_5_Encercler_C" "/Game/Blueprints/5/BP_5_MattGroupeGO.BP_5_MattGroupeGO_C"))
  (message `/Game/Blueprints/BPI_test.GetReferences` (`self.BP_Acte1Ref`) _arrayactorref)
  (bind _text (`self.SetText` "Des renforts arrivent. Les manifestants se divisent en un moyen et un plus petit groupe.   "))
  (`/Game/Blueprints/HUDClassCustom.UpdateBottomText` (`self.HudReference`) _text)
  (`self.DestroyCurrentChoices`))

(fn `UserConstructionScript`
  (`parent.UserConstructionScript`))