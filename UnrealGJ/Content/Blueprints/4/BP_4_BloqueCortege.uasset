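; BP_4_BloqueCortege is a clickable choice Blueprint in a French-language branching narrative, representing a "block the procession" option in act one.
; On click, it builds a set of three follow-up choice Blueprints and passes it to the act one Blueprint by message.
; It then updates the HUD bottom text to narrate the crowd turning violent and destroys the current choices.
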(event `self.ReceiveBeginPlay`
  (`parent.ReceiveBeginPlay`))

(event `self.TouchClick.OnClicked`
  (params (TouchedComponent :type "PrimitiveComponent Object Reference") (ButtonPressed :type "Key Structure"))
  (`KismetSystemLibrary.PrintString` "Clique Cube")
  (bind _arrayactorref (`self.SetNewChoices` 3 "/Game/Blueprints/5/BP_5_Diviser.BP_5_Diviser_C" "/Game/Blueprints/5/BP_5_Interpeller3.BP_5_Interpeller3_C" "/Game/Blueprints/5/BP_5_MattGroupe.BP_5_MattGroupe_C"))
  (message `/Game/Blueprints/BPI_test.GetReferences` (`self.BP_Acte1Ref`) _arrayactorref)
  (bind _text (`self.SetText` "La foule cherche à se défendre et devient violente"))
  (`/Game/Blueprints/HUDClassCustom.UpdateBottomText` (`self.HudReference`) _text)
  (`self.DestroyCurrentChoices`))

(fn `UserConstructionScript`
  (`parent.UserConstructionScript`))