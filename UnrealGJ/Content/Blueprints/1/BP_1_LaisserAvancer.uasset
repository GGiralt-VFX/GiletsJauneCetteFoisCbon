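; Clickable choice "LaisserAvancer" (let them advance) in Act 1 of a branching narrative, leading to the next two choices, RienDire and ParlerAvec.
; On click it passes those choices to the Act 1 Blueprint, updates the HUD's bottom text and calls MoveRight.
; After a delay it sends the choices again through QueFaireMessage, zeroes HUD blur and camera post-process weight, then destroys the current choices.
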(event `self.ReceiveBeginPlay`
  (`parent.ReceiveBeginPlay`))

(event `self.TouchClick.OnClicked`
  (params (TouchedComponent :type "PrimitiveComponent Object Reference") (ButtonPressed :type "Key Structure"))
  (`KismetSystemLibrary.PrintString` "Clique Cube")
  (bind _arrayactorref (`self.SetNewChoices` 2 "/Game/Blueprints/2/BP_2_RienDire.BP_2_RienDire_C" "/Game/Blueprints/2/BP_2_ParlerAvec.BP_2_ParlerAvec_C"))
  (message `/Game/Blueprints/BPI_test.GetReferences` (`self.BP_Acte1Ref`) _arrayactorref)
  (bind _text (`self.SetText` "Ils avancent près de vous et vous parlent"))
  (`/Game/Blueprints/HUDClassCustom.UpdateBottomText` (`self.HudReference`) _text)
  (`self.Move Right`)
  (`KismetSystemLibrary.Delay` (`self.DelayBeforeSpawn`))
  (message `/Game/Blueprints/BPI_test.QueFaire` (`self.BP_Acte1Ref`) _arrayactorref)
  (`/Game/Blueprints/HUDClassCustom.UpdateBlur` (`self.HudReference`) 0.0)
  (`CameraComponent.SetPostProcessBlendWeight` (`CameraActor.CameraComponent` (`/Game/Blueprints/BP_Acte1.Camera` (`self.BP_Acte1Ref`))) 0.0)
  (`self.DestroyCurrentChoices`))

(fn `UserConstructionScript`
  (`parent.UserConstructionScript`))