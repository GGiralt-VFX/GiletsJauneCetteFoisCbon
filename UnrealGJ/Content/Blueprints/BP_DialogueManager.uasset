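; BP_DialogueManager is a dialogue manager actor that spawns dialogue box actors when play begins.
; It loops over DialogueBoxes and spawns a new actor of each entry's class, starting from the root component's world transform.
; Each spawn is raised 100 units above the previous one, forming a vertical stack.
; GetReferences is an empty stub, and the four Choix variables are unused.
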(event `self.ReceiveBeginPlay`
  (bind _output_get (set `self.ManagerTransform` (`SceneComponent.K2_GetComponentToWorld` (`self.DefaultSceneRoot`))))
  (bind _output_get_2 (set `self.SpawnTransform` (`KismetMathLibrary.MakeTransform` (.location _output_get) (.rotation _output_get) (.scale _output_get))))
  (for _array_element (`self.dialogueBoxes`)
    (bind _output_get_3 (set `self.SpawnTransform` (`KismetMathLibrary.MakeTransform` (+ (.location _output_get_2) (0.0 0.0 100.0)) (.rotation _output_get_2) (.scale _output_get_2))))
    (`|SpawnActorFromClass` (`GameplayStatics.GetObjectClass` _array_element) _output_get_3 "Undefined" "OverrideRootScale" null null)))

(event `/Game/Blueprints/BPI_test.GetReferences`
  (params (ActorRefs :type "Array of Actor Class Reference (by ref)")))

(fn `UserConstructionScript`)