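; Act 1 manager that stages a story beat, then spawns two or three choice actors for the player.
; After a startup delay, BeginPlay sets the HUD bottom text, shifts GJ_Prefab actors, waits, then fills the choice array.
; The array length selects hardcoded choices at preset transforms, with UI blur and camera post-process for two.
; GetReferences offers an alternate entry, spawning whatever classes it receives.
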(event `self.ReceiveBeginPlay`
  (`KismetSystemLibrary.Delay` 5.0) ; Petit delay sinon il choppe pas bien la ref de l'UI
  (`self.GetHUDReference`)
  ;[1 1 1] Set du text en bas de l'écran
  (bind _output (`self.SetText` "Montext"))
  (`/Game/Blueprints/HUDClassCustom.UpdateBottomText` (`self.HUDReference`) _output)
  ;[1 1 1] ACTION (avec delay)
  (bind _outactors (`GameplayStatics.GetAllActorsOfClass` "/Game/Blueprints/GJ_Prefab.GJ_Prefab_C"))
  (for _array_element _outactors
    (`self.K2_SetActorLocation` _array_element (- (`self.K2_GetActorLocation` _array_element) (500.0 0.0 0.0)) false false)
    (`KismetSystemLibrary.Delay` (`self.delayApresAction`))
    ;[1 1 1] CHOIX (spawn des choix, blur UI etc)
    (`self.FillChoices` 2 "/Game/Blueprints/1/BP_1_LaisserAvancer.BP_1_LaisserAvancer_C")
    (switch `int` (`KismetArrayLibrary.Array_Length` (`self.ArrayActorRef`))
      (:`2`
        (`self.Spawn2Choices` "/Game/Blueprints/1/BP_1_LaisserAvancer.BP_1_LaisserAvancer_C" "/Game/Blueprints/1/BP_1_PositionBouclier.BP_1_PositionBouclier_C")
        (`/Game/Blueprints/HUDClassCustom.UpdateBlur` (`self.HUDReference`) 5.0)
        (`CameraComponent.SetPostProcessBlendWeight` (`CameraActor.CameraComponent` (`self.Camera`)) 1.0))
      (:`3`
        (`self.Spawn3Choices` "/Game/Blueprints/Choix1TestRomain/BP_Acte1_Choix1.BP_Acte1_Choix1_C" "/Game/Blueprints/Choix1TestRomain/BP_Acte1_Choix2.BP_Acte1_Choix2_C" "/Game/Blueprints/Choix1TestRomain/BP_Acte1_Choix3.BP_Acte1_Choix3_C")))))

(event `/Game/Blueprints/BPI_test.GetReferences`
  (params (ActorRefs :type "Array of Actor Class Reference (by ref)"))
  (`KismetSystemLibrary.PrintString` "Message received")
  (bind _output_get (set `self.ArrayActorRef` ActorRefs))
  (bind _returnvalue (`KismetArrayLibrary.Array_Length` _output_get))
  (`KismetSystemLibrary.PrintString` (`KismetStringLibrary.Conv_IntToString` _returnvalue))
  (switch `int` _returnvalue
    (:`2`
      (bind _output (`|GetArrayItem` _output_get))
      (bind _output_2 (`|GetArrayItem` _output_get 1))
      (`self.Spawn2Choices` _output _output_2))
    (:`3`
      (`self.Spawn3Choices` _output _output_2 (`|GetArrayItem` _output_get 2)))))

(fn `FillChoices`
  (params (NumberOfChoices :type Integer) (Choice1 :type "Actor Class Reference") (Choice2 :type "Actor Class Reference") (Choice3 :type "Actor Class Reference") (Choice4 :type "Actor Class Reference"))
  (bind _arrayactorref (`self.ArrayActorRef`))
  (`|ExecutionSequence`
    (:`then_0`
      (`KismetArrayLibrary.Array_Clear` _arrayactorref))
    (:`then_1`
      (if (>= NumberOfChoices 1)
        (`KismetArrayLibrary.Array_Add` _arrayactorref Choice1)))
    (:`then_2`
      (if (>= NumberOfChoices 2)
        (`KismetArrayLibrary.Array_Add` _arrayactorref Choice2)))
    (:`then_3`
      (if (>= NumberOfChoices 3)
        (`KismetArrayLibrary.Array_Add` _arrayactorref Choice3)))
    (:`then_4`
      (if (>= NumberOfChoices 4)
        (`KismetArrayLibrary.Array_Add` _arrayactorref Choice4)))))

(fn `GetHUDReference`
  (set `self.HUDReference` (cast `/Game/Blueprints/HUDClassCustom` (`PlayerController.GetHUD` (`GameplayStatics.GetPlayerController` 0)) :!pure true)))

(fn `SetText`
  (params (BottomText :type Text))
  (returns (Output :type Text))
  (return BottomText))

(fn `Spawn2Choices`
  (params (Choice1 :type "Actor Class Reference") (Choice2 :type "Actor Class Reference"))
  (locals (Choice1Transform :type "Transform Structure" :default "-3900.000000,4150.000000,1065.000000|19.999960,0.000000,0.000000|1.000000,1.000000,1.000000") (Choice2Transform :type "Transform Structure" :default "-4400.000000,4150.000000,880.000000|19.999960,0.000000,0.000000|1.000000,1.000000,1.000000"))
  (`|ExecutionSequence`
    (:`then_0`
      (`|SpawnActorFromClass` Choice1 (`local.Choice1Transform`) "Undefined" "OverrideRootScale" null null))
    (:`then_1`
      (`|SpawnActorFromClass` Choice2 (`local.Choice2Transform`) "Undefined" "OverrideRootScale" null null))
    (:`then_2`
      (return))))

(fn `Spawn3Choices`
  (params (Choice1 :type "Actor Class Reference") (Choice2 :type "Actor Class Reference") (Choice3 :type "Actor Class Reference"))
  (locals (Choice1Transform :type "Transform Structure" :default "-3690.000000,4150.000000,1140.000000|19.999960,0.000000,0.000000|1.000000,1.000000,1.000000") (Choice2Transform :type "Transform Structure" :default "-4174.472656,4150.000000,962.084534|19.999968,0.000000,0.000000|1.000000,1.000000,1.000000") (Choice3Transform :type "Transform Structure" :default "-4174.472656,4150.000000,962.084534|19.999960,0.000000,0.000000|1.000000,1.000000,1.000000"))
  (`|ExecutionSequence`
    (:`then_0`
      (`|SpawnActorFromClass` Choice1 (`local.Choice1Transform`) "Undefined" "OverrideRootScale" null null))
    (:`then_1`
      (`|SpawnActorFromClass` Choice2 (`local.Choice2Transform`) "Undefined" "OverrideRootScale" null null))
    (:`then_2`
      (`|SpawnActorFromClass` Choice3 (`local.Choice3Transform`) "Undefined" "OverrideRootScale" null null))))

(fn `UserConstructionScript`)