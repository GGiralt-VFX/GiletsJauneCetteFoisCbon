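; BP_2_LancerLac is a clickable choice in a branching riot-police narrative, where protesters throw stones and injure an officer.
; On touch click, it registers three follow-up choices (water cannon, flashball, defensive position) with the act-one blueprint reference.
; It then updates the HUD bottom text with the French outcome and destroys the current choices.
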(event `self.ReceiveBeginPlay`
  (`parent.ReceiveBeginPlay`))

(event `self.TouchClick.OnClicked`
  (params (TouchedComponent :type "PrimitiveComponent Object Reference") (ButtonPressed :type "Key Structure"))
  (`KismetSystemLibrary.PrintString` "Clique Cube")
  (bind _arrayactorref (`self.SetNewChoices` 3 "/Game/Blueprints/3/BP_3_ChaufferCanonEau.BP_3_ChaufferCanonEau_C" "/Game/Blueprints/3/BP_3_Flashball.BP_3_Flashball_C" "/Game/Blueprints/3/BP_3_PosDefensive.BP_3_PosDefensive_C"))
  (message `/Game/Blueprints/BPI_test.GetReferences` (`self.BP_Acte1Ref`) _arrayactorref)
  (bind _text (`self.SetText` "Les manifestant lancent des cailloux et des briques. Un de vos CRS est blessé "))
  (`/Game/Blueprints/HUDClassCustom.UpdateBottomText` (`self.HudReference`) _text)
  (`self.DestroyCurrentChoices`))

(fn `UserConstructionScript`
  (`parent.UserConstructionScript`))